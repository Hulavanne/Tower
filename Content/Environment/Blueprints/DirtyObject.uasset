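; DirtyObject is a washable prop that switches from a dirty to a clean material when the player casts a water spell on it.
; Overlap events track whether a PlayerCharacter is in range, and Tick clears Dirty if that player is casting during the overlap.
; Tick reapplies the dirty material while dirty and sets the clean one once afterward.
; The construction script previews either state; an alpha timeline material fade is left unconnected.
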(event Collision|EventActorBeginOverlap
  (params (OtherActor :type Actor%20Object%20Reference))
  ;[1 1 1] Setting isOverlapping
  (if (Utilities|ClassIsChildOf (Utilities|GetClass OtherActor) "/Game/Player/Blueprints/PlayerCharacter.PlayerCharacter_C")
    (Variables|Default|SetisOverlapping true)))

(event Collision|EventActorEndOverlap
  (params (OtherActor :type Actor%20Object%20Reference))
  ;[1 1 1] Setting isOverlapping
  (if (Utilities|ClassIsChildOf (Utilities|GetClass OtherActor) "/Game/Player/Blueprints/PlayerCharacter.PlayerCharacter_C")
    (Variables|Default|SetisOverlapping false)))

(event EventTick
  (params (DeltaSeconds :type Float%20%28single-precision%29))
  (bind _staticmeshcomponent (Variables|Debug|GetStaticMeshComponent))
  ;[1 1 1] Washing the object
  (if (Variables|Default|Getdirty)
    (Rendering|Material|SetMaterial _staticmeshcomponent 0 (Variables|Default|GetdirtyMaterial))
    (if (Variables|Default|GetisOverlapping)
      (bind _asplayer_character (Utilities|Casting|CastToPlayerCharacter (Game|Player|GetPlayerPawn 0)))
      (if (Variables|/Game/Player/Blueprints/PlayerCharacter.PlayerCharacter_C|GetcastingWaterSpell _asplayer_character)
        (Variables|Default|Setdirty false)))
    (else
      (Utilities|FlowControl|DoOnce false
        (:Completed
          (Rendering|Material|SetMaterial _staticmeshcomponent 0 (Variables|Default|GetcleanMaterial)))))))

(fn ConstructionScript
  (if (Variables|Default|Getdirty)
    (Rendering|Material|SetMaterial (Variables|Debug|GetStaticMeshComponent) 0 (Variables|Default|GetdirtyMaterial))
    (else
      (Rendering|Material|SetMaterial (Variables|Debug|GetStaticMeshComponent) 0 (Variables|Default|GetcleanMaterial)))))
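; Flammable environment object that the player lights with a fire spell and puts out with a water spell.
; Overlap events track when a PlayerCharacter is in range, and Tick then checks that pawn's casting flags to toggle FireOn.
; Dousing swaps the Fire effect for Steam, which switches off after a short delay.
; The construction script starts the fire effect when FireOn is preset.
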(event Collision|EventActorBeginOverlap
  (params (OtherActor :type Actor%20Object%20Reference))
  ;[1 1 1] Setting isOverlapping
  (if (Utilities|ClassIsChildOf (Utilities|GetClass OtherActor) "/Game/Player/Blueprints/PlayerCharacter.PlayerCharacter_C")
    (Variables|Default|SetisOverlapping true)))

(event Collision|EventActorEndOverlap
  (params (OtherActor :type Actor%20Object%20Reference))
  ;[1 1 1] Setting isOverlapping
  (if (Utilities|ClassIsChildOf (Utilities|GetClass OtherActor) "/Game/Player/Blueprints/PlayerCharacter.PlayerCharacter_C")
    (Variables|Default|SetisOverlapping false)))

(event EventTick
  (params (DeltaSeconds :type Float%20%28single-precision%29))
  ;[1 1 1] If fire is not already on, activate the effects
  (if (Variables|Default|GetFireOn)
    (Components|Activation|Activate (Variables|Default|GetFire) false)
    (Components|Activation|Deactivate (Variables|Default|GetSteam))
    ;[1 1 1] If water spell is being used on the object, deactivate fire effects and activate steam
    (if (Variables|Default|GetisOverlapping)
      (bind _asplayer_character (Utilities|Casting|CastToPlayerCharacter (Game|Player|GetPlayerPawn 0)))
      (if (Variables|/Game/Player/Blueprints/PlayerCharacter.PlayerCharacter_C|GetcastingWaterSpell _asplayer_character)
        (Components|Activation|Activate (Variables|Default|GetSteam) false)
        (Components|Activation|Deactivate (Variables|Default|GetFire))
        (Variables|Default|SetFireOn false)
        ;[1 1 1] Deactivate the steam after a while
        (Utilities|FlowControl|RetriggerableDelay 5.0)
        (Components|Activation|Deactivate (Variables|Default|GetSteam))))
    (elif (Variables|Default|GetisOverlapping)
      (bind _asplayer_character_2 (Utilities|Casting|CastToPlayerCharacter (Game|Player|GetPlayerPawn 0)))
      (if (Variables|/Game/Player/Blueprints/PlayerCharacter.PlayerCharacter_C|GetcastingFireSpell _asplayer_character_2)
        (Variables|Default|SetFireOn true)))))

(fn ConstructionScript
  (if (Variables|Default|GetFireOn)
    (Components|Activation|Activate (Variables|Default|GetFire) false)))
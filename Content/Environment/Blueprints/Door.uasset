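; Door actor for spline-based movement that configures its spline, its position along it and its paired door at construction time.
; Unless set manually, it picks the nearest MovementSpline through a recursive closest-point search, then stores its distance along that spline.
; The GetClosestDoor bool acts as a one-shot editor button, resetting itself and linking the nearest other Door as CounterpartDoor.
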(event EventTick
  (params (DeltaSeconds :type Float%20%28single-precision%29)))

(fn ConstructionScript
  (CallFunction|SetNearestSpline (Variables|Default|Getspline))
  (CallFunction|SetPositionAlongSpline)
  (CallFunction|SetCounterpartDoor))

(fn SetNearestSpline
  (params (NewParam :type Movement%20Spline%20Object%20Reference%20%28by%20ref%29))
  (if (not (Variables|Default|GetsetSplineManually))
    ;[1 1 1] Get a list of all splines in the level
    (bind _outactors (Actor|GetAllActorsOfClass "/Game/Player/Blueprints/MovementSpline.MovementSpline_C"))
    (for _array_element _outactors
      ;[1 1 1] Get the nearest location on each spline in realtion to the position of this object and add its distance to the object to a list
      (bind _besttime (Default|RecursiveDistanceCheck _array_element (Variables|/Game/Player/Blueprints/MovementSpline.MovementSpline_C|GetplayerSpline _array_element) (Transformation|GetActorLocation) 100 0.0 1.0 true))
      (Utilities|Array|Add (LocalVariables|Getdistances) (Math|Vector|VectorLength (- (Spline|GetLocationatTime (Variables|/Game/Player/Blueprints/MovementSpline.MovementSpline_C|GetplayerSpline _array_element) _besttime "World" (Variables|/Game/Player/Blueprints/MovementSpline.MovementSpline_C|GetconstantVelocity _array_element)) (Transformation|GetActorLocation)))))
    ;[1 1 1] Get the shortest distance from the list and set its owner to be the spline
    (|SetBy-RefVar NewParam (Utilities|Array|Get(acopy) _outactors (.IndexOfMinValue (Math|Float|MinOfFloatArray (LocalVariables|Getdistances)))))))

(fn SetPositionAlongSpline
  (bind _spline (Variables|Default|Getspline))
  (Utilities|IsValid _spline
    (:Is%20Valid
      (bind _besttime (Default|RecursiveDistanceCheck _spline (Variables|/Game/Player/Blueprints/MovementSpline.MovementSpline_C|GetplayerSpline _spline) (Transformation|GetActorLocation) 30 0.0 1.0 false))
      (bind _distance (Default|ConvertTimetoDistance (Variables|Default|Getspline) _besttime))
      (Variables|Default|SetpositionAlongSpline _distance))))

(fn SetCounterpartDoor
  (if (Variables|Default|GetgetClosestDoor)
    (Variables|Default|SetgetClosestDoor false)
    (LocalVariables|Setindex 0)
    (LocalVariables|Setdistance 1e+05)
    (bind _outactors (Actor|GetAllActorsOfClass "Door_C"))
    (for (_array_element _array_index) _outactors
      (if (not (== self _array_element))
        (if (> (LocalVariables|Getdistance) (Math|Vector|VectorLength (- (Transformation|GetActorLocation _array_element) (Transformation|GetActorLocation))))
          (LocalVariables|Setindex _array_index)
          (LocalVariables|Setdistance (Math|Vector|VectorLength (- (Transformation|GetActorLocation _array_element) (Transformation|GetActorLocation)))))))
    (Variables|Default|SetcounterpartDoor (Utilities|Array|Get(acopy) _outactors (LocalVariables|Getindex)))))
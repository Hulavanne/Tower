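; LevelEndingGate is an environment gate actor that ends the current level by loading IndoorsLevel when the player interacts with it.
; Collider begin and end overlap events track whether a PlayerCharacter is inside.
; While that overlap flag is set, Tick polls the player character's Interact flag and opens the hard-coded level by name when it is true.
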(event OnComponentBeginOverlap(collider)
  (params (OtherActor :type Actor%20Object%20Reference) (OtherComp :type Primitive%20Component%20Object%20Reference) (OtherBodyIndex :type Integer) (bFromSweep :type Boolean) (SweepResult :type Hit%20Result%20Structure%20%28by%20ref%29))
  ;[1 1 1] Setting isOverlapping
  (if (Utilities|ClassIsChildOf (Utilities|GetClass OtherActor) "/Game/Player/Blueprints/PlayerCharacter.PlayerCharacter_C")
    (Variables|Default|SetplayerOverlapping true)))

(event OnComponentEndOverlap(collider)
  (params (OtherActor :type Actor%20Object%20Reference) (OtherComp :type Primitive%20Component%20Object%20Reference) (OtherBodyIndex :type Integer))
  ;[1 1 1] Setting isOverlapping
  (if (Utilities|ClassIsChildOf (Utilities|GetClass OtherActor) "/Game/Player/Blueprints/PlayerCharacter.PlayerCharacter_C")
    (Variables|Default|SetplayerOverlapping false)))

(event EventTick
  (params (DeltaSeconds :type Float%20%28single-precision%29))
  (if (Variables|Default|GetplayerOverlapping)
    (bind _asplayer_character (Utilities|Casting|CastToPlayerCharacter (Game|GetPlayerCharacter 0)))
    (if (Variables|/Game/Player/Blueprints/PlayerCharacter.PlayerCharacter_C|Getinteract _asplayer_character)
      (Game|OpenLevel(byName) "IndoorsLevel"))))

(fn ConstructionScript)
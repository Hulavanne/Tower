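; Pickup is a physics actor that the player can pick up and drop with the interact input.
; Mesh overlap events flag when the player character is in range, and Tick polls the player's Interact flag.
; Pickup requires empty hands and grounded footing, then grabs the mesh through the player's physics handle and updates carry state on both actors.
; Dropping releases the handle and optionally zeroes the mesh's linear velocity.
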(event OnComponentBeginOverlap(StaticMeshComponent)
  (params (OtherActor :type Actor%20Object%20Reference) (OtherComp :type Primitive%20Component%20Object%20Reference) (OtherBodyIndex :type Integer) (bFromSweep :type Boolean) (SweepResult :type Hit%20Result%20Structure%20%28by%20ref%29))
  ;[1 1 1] Checking for collisions with the player
  (if (Utilities|ClassIsChildOf (Utilities|GetClass OtherActor) "/Game/Player/Blueprints/PlayerCharacter.PlayerCharacter_C")
    (if (not (Variables|Default|GetbeingCarried))
      (Variables|Default|Setcolliding true))))

(event OnComponentEndOverlap(StaticMeshComponent)
  (params (OtherActor :type Actor%20Object%20Reference) (OtherComp :type Primitive%20Component%20Object%20Reference) (OtherBodyIndex :type Integer))
  ;[1 1 1] Checking for collisions with the player
  (if (Utilities|ClassIsChildOf (Utilities|GetClass OtherActor) "/Game/Player/Blueprints/PlayerCharacter.PlayerCharacter_C")
    (if (not (Variables|Default|GetbeingCarried))
      (Variables|Default|Setcolliding false))))

(event EventTick
  (params (DeltaSeconds :type Float%20%28single-precision%29))
  (bind _player (Variables|Default|Getplayer))
  (bind _player_2 (Variables|Default|Getplayer))
  (bind _player_3 (Variables|Default|Getplayer))
  (bind _staticmeshcomponent (Variables|Debug|GetStaticMeshComponent))
  (if (Variables|Default|GetbeingCarried)
    ;[1 1 1] Check for input
    (if (Variables|/Game/Player/Blueprints/PlayerCharacter.PlayerCharacter_C|Getinteract _player_3)
      ;[1 1 1] Drop item
      (Variables|/Game/Player/Blueprints/PlayerCharacter.PlayerCharacter_C|Setinteract _player_3 false)
      (Variables|/Game/Player/Blueprints/PlayerCharacter.PlayerCharacter_C|SetcarryingItem _player_3 false)
      (Physics|Components|PhysicsHandle|ReleaseComponent (Variables|/Game/Player/Blueprints/PlayerCharacter.PlayerCharacter_C|GetPlayerPhysicsHandle _player_3))
      (Variables|Default|SetbeingCarried false)
      ;[1 1 1] Comment
      (if (Variables|Default|GetconstrainWhenDropped)
        (Physics|SetPhysicsLinearVelocity (Variables|Debug|GetStaticMeshComponent) "0, 0, 0" false "None")))
    (elif (not (or (Variables|/Game/Player/Blueprints/PlayerCharacter.PlayerCharacter_C|GetcarryingItem _player) (Variables|/Game/Player/Blueprints/PlayerCharacter.PlayerCharacter_C|GetisInAir _player)))
      (if (Variables|Default|Getcolliding)
        ;[1 1 1] Check for input
        (if (Variables|/Game/Player/Blueprints/PlayerCharacter.PlayerCharacter_C|Getinteract _player_2)
          ;[1 1 1] Pick the item up
          (Variables|/Game/Player/Blueprints/PlayerCharacter.PlayerCharacter_C|Setinteract _player_2 false)
          (Variables|/Game/Player/Blueprints/PlayerCharacter.PlayerCharacter_C|SetcarryingItem _player_2 true)
          (Variables|/Game/Player/Blueprints/PlayerCharacter.PlayerCharacter_C|SetitemBeingCarried _player_2 self)
          (Class|PhysicsHandleComponent|GrabComponent (Variables|/Game/Player/Blueprints/PlayerCharacter.PlayerCharacter_C|GetPlayerPhysicsHandle _player_2) _staticmeshcomponent "None" (Transformation|GetWorldLocation _staticmeshcomponent) false)
          (Variables|Default|Setcolliding false)
          (Variables|Default|SetbeingCarried true))))))

(event EventBeginPlay
  (bind _asplayer_character (Utilities|Casting|CastToPlayerCharacter (Game|Player|GetPlayerPawn 0)))
  (Variables|Default|Setplayer _asplayer_character))

(fn ConstructionScript)
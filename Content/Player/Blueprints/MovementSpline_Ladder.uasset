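; Ladder movement spline for the player, which builds its mesh and trigger and links to neighbouring movement splines.
; The construction script adds a spline mesh per segment and sizes and positions the trigger box from segment midpoint height.
; Unless splines are set manually, SetNearestSpline searches the player character's SplinesInLevel with RecursiveDistanceCheck, assigning the closest to the top and bottom points as SplineAbove and SplineBelow.
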(event EventBeginPlay)

(event EventActorBeginOverlap
  (params (OtherActor :type Actor%20Object%20Reference)))

(event EventTick
  (params (DeltaSeconds :type Float%20%28single-precision%29))
  (|CallParentFunction 0.0))

(fn ConstructionScript
  (bind _trigger (Variables|Default|Gettrigger))
  (bind _arrow (Variables|Default|Getarrow))
  (bind _playerspline (Variables|Default|GetplayerSpline))
  (bind _relativelocation (Variables|/Script/Engine.SceneComponent|GetRelativeLocation _arrow))
  (|CallParentFunction)
  ;[1 1 1] Spwning the ladder mesh
  (for _index (range 0 (- (Spline|GetNumberOfSplinePoints (Variables|Default|GetplayerSpline)) 2))
    (bind _returnvalue (AddComponent|AddSplineMeshComponent true (Math|Transform|MakeTransform (Variables|/Script/Engine.SceneComponent|GetRelativeLocation (Variables|Default|Getarrow)) "0, 0, 0" (Math|Vector|MakeVector (LocalVariables|GetscaleX) 1.0 1.0))))
    (Class|SceneComponent|Attachto _returnvalue (Variables|Default|GetplayerSpline) "None" "KeepRelativeOffset" true)
    (SplineMesh|SetStartandEnd _returnvalue (.Location (Spline|GetLocationandTangentatSplinePoint _playerspline _index "Local")) (.Tangent (Spline|GetLocationandTangentatSplinePoint _playerspline _index "Local")) (.Location (Spline|GetLocationandTangentatSplinePoint _playerspline (+ _index 1) "Local")) (.Tangent (Spline|GetLocationandTangentatSplinePoint _playerspline (+ _index 1) "Local")) :!class /Script/Engine.SplineMeshComponent)
    ;[1 1 1] Extending the trigger box to the length of the ladder
    (Components|Box|SetBoxExtent _trigger (Math|Vector|MakeVector 1e+02 1.0 (.z (Math|Vector|Lerp(Vector) (.Location (Spline|GetLocationandTangentatSplinePoint _playerspline _index "Local")) (.Location (Spline|GetLocationandTangentatSplinePoint _playerspline (+ _index 1) "Local")) 0.5))) true)
    (Transformation|SetRelativeTransform _trigger (Math|Transform|MakeTransform (Math|Vector|MakeVector (.x _relativelocation) (.y _relativelocation) (.z (Math|Vector|Lerp(Vector) (.Location (Spline|GetLocationandTangentatSplinePoint _playerspline _index "Local")) (.Location (Spline|GetLocationandTangentatSplinePoint _playerspline (+ _index 1) "Local")) 0.5)))) false false))
  ;[1 1 1] Setting splineAbove and splineBelow
  (CallFunction|SetNearestSpline (Variables|Spline|GetsplineAbove) true)
  (CallFunction|SetNearestSpline (Variables|Spline|GetsplineBelow) false))

(fn SetNearestSpline
  (params (splineToBeSet :type Movement%20Spline%20Object%20Reference) (settingSplineAbove :type Boolean))
  (LocalVariables|Setspline splineToBeSet)
  (if settingSplineAbove
    (LocalVariables|Setindex (- (Spline|GetNumberOfSplinePoints (Variables|Default|GetplayerSpline)) 1))
    (else
      (LocalVariables|Setindex 0)))
  (if (not (Variables|Spline|GetsetSplinesManually))
    ;[1 1 1] Get a list of all splines in the level from the player blueprint
    (bind _outactors (Actor|GetAllActorsOfClass "/Game/Player/Blueprints/PlayerCharacter.PlayerCharacter_C"))
    (Utilities|IsValid (Utilities|Array|Get(acopy) _outactors)
      (:Is%20Valid
        (bind _output_get (LocalVariables|Setsplines (Variables|/Game/Player/Blueprints/PlayerCharacter.PlayerCharacter_C|GetsplinesInLevel (Utilities|Array|Get(acopy) _outactors))))
        (for _array_element _output_get
          ;[1 1 1] Remove self from the list
          (if (== _array_element self)
            (Utilities|Array|RemoveItem _output_get 0)
            (else
              ;[1 1 1] Get the nearest location on each spline in realtion to the position of this object and add its distance to the object to a list
              (bind _besttime (Default|RecursiveDistanceCheck _array_element (Spline|GetLocationatSplinePoint (Variables|Default|GetplayerSpline) (LocalVariables|Getindex) "World") 100 0.0 1.0 true))
              (Utilities|Array|Add (LocalVariables|Getdistances) (Math|Vector|VectorLength (- (Spline|GetLocationatTime (Variables|/Game/Player/Blueprints/MovementSpline.MovementSpline_C|GetplayerSpline _array_element) _besttime "World" (Variables|/Game/Player/Blueprints/MovementSpline.MovementSpline_C|GetconstantVelocity _array_element)) (Spline|GetLocationatSplinePoint (Variables|Default|GetplayerSpline) (LocalVariables|Getindex) "World")))))))
        ;[1 1 1] Get the shortest distance from the list and set its owner to be the spline
        (if settingSplineAbove
          (Variables|Spline|SetsplineAbove (Utilities|Array|Get(acopy) (LocalVariables|Getsplines) (.IndexOfMinValue (Math|Float|MinOfFloatArray (LocalVariables|Getdistances)))))
          (else
            (Variables|Spline|SetsplineBelow (Utilities|Array|Get(acopy) (LocalVariables|Getsplines) (.IndexOfMinValue (Math|Float|MinOfFloatArray (LocalVariables|Getdistances)))))))))))
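; Spline-rail follow camera that tracks the player's progress along PlayerSpline and moves to the matching time on CameraSpline while activated.
; Each tick, a recursive bisection approximates the player's nearest spline time, which the current time eases toward, snapping on large gaps.
; The camera interpolates to that point and turns toward a spot ahead of the player.
; Construction scrubs a camera preview; optional debug shows point numbers and spheres.
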(event EventBeginPlay)

(event Collision|EventActorBeginOverlap
  (params (OtherActor :type Actor%20Object%20Reference)))

(event EventTick
  (params (DeltaSeconds :type Float%20%28single-precision%29))
  (Variables|Default|SetdeltaTime DeltaSeconds)
  (Utilities|IsValid (Variables|Default|Getplayer)
    (:Is%20Valid
      (bind _besttime (Spline|RecursiveDistanceCheck (Variables|Spline|GetsplineIterationMax) 0.0 1.0))
      (Variables|Spline|SetsplineDesiredTime _besttime)
      (Spline|UpdateDesiredTime)
      (Camera|UpdateCamera)
      (DebugTools|DebugSplineMovement))))

(fn ConstructionScript
  (DebugTools|ScrubCameraTime)
  (DebugTools|SetupDebugNumbers))

(fn ActivateCamera
  (params (Player :type Pawn%20Object%20Reference))
  (Utilities|IsValid Player
    (:Is%20Valid
      (Variables|Default|Setplayer Player))))

(fn DeactivateCamera
  (Variables|Default|Setplayer 0))

(fn SetupDebugNumbers
  (if (Variables|DebugTools|GetshowDebug)
    (Utilities|FlowControl|Sequence
      (:then_0
        (DebugTools|AddSplineNumbers (Variables|Spline|GetPlayerSpline)))
      (:then_1
        (DebugTools|AddSplineNumbers (Variables|Spline|GetCameraSpline))))))

(fn UpdateCamera
  (bind _player (Variables|Default|Getplayer))
  (Transformation|SetWorldLocationAndRotation (Variables|Camera|GetCamera) (Math|Interpolation|VInterpTo (Transformation|GetWorldLocation (Variables|Camera|GetCamera)) (Variables|Camera|GetcameraDesiredLocation) (Variables|Default|GetdeltaTime) (Variables|Camera|GetcameraMovementInterpSpeed)) (Math|Interpolation|RInterpTo (Transformation|GetWorldRotation (Variables|Camera|GetCamera)) (Math|Rotator|FindLookatRotation (Transformation|GetWorldLocation (Variables|Camera|GetCamera)) (+ (Transformation|GetActorLocation _player) (* (Transformation|GetActorForwardVector _player) 1e+02))) (Variables|Default|GetdeltaTime) (Variables|Camera|GetcameraRotationInterpSpeed)) false false))

(fn AddSplineNumbers
  (params (Spline :type Spline%20Component%20Object%20Reference))
  (for _index (range 0 (- (Spline|GetNumberOfSplinePoints Spline) 1))
    (bind _returnvalue (AddComponent|AddTextRenderComponent false (Math|Transform|MakeTransform (+ (.Location (Spline|GetLocationandTangentatSplinePoint Spline _index "Local")) "0, 0,20.000000") (Math|Rotator|CombineRotators (Math|Rotator|MakeRotfromX (.Tangent (Spline|GetLocationandTangentatSplinePoint Spline _index "Local"))) "0,180.000000, 0"))))
    (Rendering|Components|TextRender|SetText _returnvalue (Utilities|Text|ToText(Integer) _index))))

(fn DebugSplineMovement
  (if (Variables|DebugTools|GetshowDebug)
    (Rendering|Debug|DrawDebugSphere (Spline|GetLocationatTime (Variables|Spline|GetPlayerSpline) (Variables|Spline|GetsplineCurrentTime) "World" (Variables|Spline|GetconstantVelocity)) 5e+01 12 "(R=1.000000,G=0.000000,B=0.000000,A=1.000000)" 0.0)
    (Rendering|Debug|DrawDebugSphere (Spline|GetLocationatTime (Variables|Spline|GetPlayerSpline) (Variables|Spline|GetsplineDesiredTime) "World" (Variables|Spline|GetconstantVelocity)) 5e+01 12 "(R=1.000000,G=0.000000,B=0.000000,A=1.000000)" 0.0)
    (Rendering|Debug|DrawDebugSphere (Spline|GetLocationatTime (Variables|Spline|GetCameraSpline) (Variables|Spline|GetsplineCurrentTime) "World" (Variables|Spline|GetconstantVelocity)) 5e+01 12 "(R=0.079714,G=1.000000,B=0.000000,A=1.000000)" 0.0)
    (Rendering|Debug|DrawDebugSphere (Spline|GetLocationatTime (Variables|Spline|GetCameraSpline) (Variables|Spline|GetsplineDesiredTime) "World" (Variables|Spline|GetconstantVelocity)) 5e+01 12 "(R=0.079714,G=1.000000,B=0.000000,A=1.000000)" 0.0)))

(fn ScrubCameraTime
  (bind _playerspline (Variables|Spline|GetPlayerSpline))
  (bind _cameraspline (Variables|Spline|GetCameraSpline))
  (bind _cameradebugtime (Variables|DebugTools|GetcameraDebugTime))
  (bind _constantvelocity (Variables|Spline|GetconstantVelocity))
  (bind _returnvalue (Spline|GetLocationatTime _playerspline _cameradebugtime "World" _constantvelocity))
  (bind _returnvalue_2 (Spline|GetLocationatTime _cameraspline _cameradebugtime "World" _constantvelocity))
  (bind _returnvalue_3 (Math|Rotator|FindLookatRotation _returnvalue_2 _returnvalue))
  (Transformation|SetWorldLocationAndRotation (Variables|Camera|GetCamera) _returnvalue_2 (Math|Rotator|MakeRotator (.roll _returnvalue_3) (.pitch _returnvalue_3) 0.0) false false))

(fn RecursiveDistanceCheck
  (params (iteration :type Integer) (startTime :type Float%20%28single-precision%29) (endTime :type Float%20%28single-precision%29))
  (bind _playerspline (Variables|Spline|GetPlayerSpline))
  (bind _constantvelocity (Variables|Spline|GetconstantVelocity))
  (bind _player (Variables|Default|Getplayer))
  (bind _returnvalue (Transformation|GetActorLocation _player))
  (LocalVariables|Setindex iteration)
  (LocalVariables|Setstart startTime)
  (LocalVariables|Setend endTime)
  (LocalVariables|SetstartDistance (Math|Vector|VectorLength (- (Spline|GetLocationatTime _playerspline (LocalVariables|Getstart) "World" _constantvelocity) _returnvalue)))
  (LocalVariables|SetendDistance (Math|Vector|VectorLength (- (Spline|GetLocationatTime _playerspline (LocalVariables|Getend) "World" _constantvelocity) _returnvalue)))
  (if (< (LocalVariables|GetstartDistance) (LocalVariables|GetendDistance))
    (if (<= (LocalVariables|Getindex) 0)
      (LocalVariables|Setbest (LocalVariables|Getstart) :!label _label)
      (else
        (LocalVariables|Setindex (- (LocalVariables|Getindex) 1))
        (if (<= (LocalVariables|GetstartDistance) (Variables|Spline|GetdistanceThreshold))
          (goto _label)
          (else
            (bind _besttime (Spline|RecursiveDistanceCheck (LocalVariables|Getindex) (LocalVariables|Getstart) (Math|Float|Lerp (LocalVariables|Getstart) (LocalVariables|Getend) 0.5)))
            (LocalVariables|Setbest _besttime)))))
    (elif (<= (LocalVariables|Getindex) 0)
      (LocalVariables|Setbest (LocalVariables|Getend) :!label _label_2)
      (else
        (LocalVariables|Setindex (- (LocalVariables|Getindex) 1))
        (if (<= (LocalVariables|GetendDistance) (Variables|Spline|GetdistanceThreshold))
          (goto _label_2)
          (else
            (bind _besttime_2 (Spline|RecursiveDistanceCheck (LocalVariables|Getindex) (Math|Float|Lerp (LocalVariables|Getstart) (LocalVariables|Getend) 0.5) (LocalVariables|Getend)))
            (LocalVariables|Setbest _besttime_2))))))
  (return (LocalVariables|Getbest)))

(fn UpdateDesiredTime
  (if (>= (Math|Float|Absolute(Float) (- (Variables|Spline|GetsplineDesiredTime) (Variables|Spline|GetsplineCurrentTime))) (Variables|Spline|GettimeDifferenceThreshold))
    (Variables|Spline|SetsplineCurrentTime (Variables|Spline|GetsplineDesiredTime))
    (else
      (Variables|Spline|SetsplineCurrentTime (+ (* (- (Variables|Spline|GetsplineDesiredTime) (Variables|Spline|GetsplineCurrentTime)) (Variables|Default|GetdeltaTime) (Variables|Camera|GetcameraSpeed)) (Variables|Spline|GetsplineCurrentTime)))))
  (Variables|Camera|SetcameraDesiredLocation (Spline|GetLocationatTime (Variables|Spline|GetCameraSpline) (Variables|Spline|GetsplineCurrentTime) "World" (Variables|Spline|GetconstantVelocity))))
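; Game HUD that draws a line of dialog text on screen, centered horizontally in the lower part of the view.
; DrawTextDialog stores the text and opens a gate, and StopTextDialog closes it.
; DrawHUD enters that gate every frame, so the text is redrawn while the gate is open, positioned from screen size and measured text size.
; An unconnected DrawLine node never runs.
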(event Custom|Draw%20Text%20Dialog
  (params (text :type String))
  (Variables|Default|Settext text)
  (Utilities|FlowControl|Gate true) ; enters at Open
)

(event Custom|Stop%20Text%20Dialog
  (bind _textsize (Variables|Default|GettextSize))
  (bind _font (Variables|Default|Getfont))
  (bind _text (Variables|Default|Gettext))
  (bind (_outwidth _outheight) (Class|HUD|GetTextSize _text _font _textsize))
  (Utilities|FlowControl|Gate true) ; enters at Close
)

(event EventTick
  (params (DeltaSeconds :type Float%20%28single-precision%29)))

(event EventDrawHUD
  (params (SizeX :type Integer) (SizeY :type Integer))
  (bind _textsize (Variables|Default|GettextSize))
  (bind _font (Variables|Default|Getfont))
  (bind _text (Variables|Default|Gettext))
  (bind (_outwidth _outheight) (Class|HUD|GetTextSize _text _font _textsize))
  (Utilities|FlowControl|Gate true
    (:Exit
      (HUD|DrawText _text (Variables|Default|GettextColor) (- (* SizeX 0.5) (* _outwidth 0.5)) (- (* SizeY 0.8) (* _outheight 0.5)) (Variables|Default|Getfont) (Variables|Default|GettextSize) false))))

(fn ConstructionScript)